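; Lobby player controller for a multiplayer session, handling the lobby UI, player roster, chat and session exit.
; On local BeginPlay it creates the lobby widget and spawns and possesses a PCH_Game pawn with the saved name and a timestamp-built ID.
; Spawning rebuilds the roster from the game mode's controller list and pushes it to each controller's widget; chat fans out likewise.
; Other events set the game state's map index and show a loading screen.
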(event `self.ReceiveBeginPlay`
  (if (`self.IsLocalPlayerController`)
    (bind _returnvalue (`|CreateWidget` "/Game/Assets/UMG/UMG_Lobby.UMG_Lobby_C" self))
    (`UserWidget.AddToViewport` _returnvalue 0)
    (set `self.UMG_Lobby` _returnvalue)
    (set `self.bShowMouseCursor` true)
    (bind _asgi_main (cast `/Game/Assets/Gameplay/GI_Main` (`GameplayStatics.GetGameInstance`)))
    (`self.EVE_Spawn_Player` (`/Game/Assets/Gameplay/GI_Main.PlayerName` _asgi_main))))

(event `EVE_Spawn_Player`
  (params (PlayerName :type Text))
  (bind (_returnvalue_year _returnvalue_month _returnvalue_day _returnvalue_hour _returnvalue_minute _returnvalue_second _returnvalue_millisecond) (`KismetMathLibrary.BreakDateTime` (`KismetMathLibrary.Now`)))
  (bind _returnvalue (`GameplayStatics.GetActorOfClass` "/Script/Engine.PlayerStart"))
  (bind _returnvalue_2 (`|SpawnActorFromClass` "/Game/Assets/Gameplay/PCH_Game.PCH_Game_C" (`self.GetTransform` _returnvalue) "Undefined" "OverrideRootScale" null (`KismetStringLibrary.Concat_StrStr` (`KismetStringLibrary.Conv_IntToString` _returnvalue_year) (`KismetStringLibrary.Conv_IntToString` _returnvalue_month) (`KismetStringLibrary.Conv_IntToString` _returnvalue_day) (`KismetStringLibrary.Conv_IntToString` _returnvalue_hour) (`KismetStringLibrary.Conv_IntToString` _returnvalue_minute) (`KismetStringLibrary.Conv_IntToString` _returnvalue_second) (`KismetStringLibrary.Conv_IntToString` _returnvalue_millisecond)) PlayerName 0 null))
  (`self.Possess` self _returnvalue_2)
  (`self.FUN_Update_Player`))

(event `EVE_Update_Map`
  (params (MapIndex :type Integer))
  (bind _asgs_lobby (cast `/Game/Assets/Gameplay/GS_Lobby` (`GameplayStatics.GetGameState`)))
  (set `/Game/Assets/Gameplay/GS_Lobby.MapIndex` MapIndex _asgs_lobby))

(event `EVE_Client_Update_Player`
  (params (Names :type "Array of Text (by ref)") (Ids :type "Array of String (by ref)"))
  (`/Game/Assets/UMG/UMG_Lobby.FUN_Update_Player` (`self.UMG_Lobby`) Names Ids))

(event `EVE_Client_Quit_Session`
  (`DestroySessionCallbackProxy.DestroySession` self
    (:`OnSuccess`
      (`GameplayStatics.OpenLevelBySoftObjectPtr` "/Game/Assets/Maps/MainMenu.MainMenu"))))

(event `EVE_Server_Add_Message`
  (params (InText :type Text))
  (bind _asgm_lobby (cast `/Game/Assets/Gameplay/GM_Lobby` (`GameplayStatics.GetGameMode`)))
  (for _array_element (`/Game/Assets/Gameplay/GM_Lobby.PcList` _asgm_lobby)
    (`self.EVE_Client_Add_Message` _array_element InText)))

(event `EVE_Client_Add_Message`
  (params (InText :type Text))
  (`/Game/Assets/UMG/UMG_Lobby.FUN_Add_Message` (`self.UMG_Lobby`) InText))

(event `EVE_Client_Loding`
  (`/Maple_FastSetting/Library/FUNL_FastSetting.FUNL_FastCreateWidget` "/Maple_FastSetting/UMG/Loading/UMG_Loading_OnlyText.UMG_Loading_OnlyText_C" 10))

(fn `FUN_Update_Player`
  (locals (Names :type "Array of Text") (IDs :type "Array of String"))
  (for _array_element (`/Game/Assets/Gameplay/GM_Lobby.PcList` (cast `/Game/Assets/Gameplay/GM_Lobby` (`GameplayStatics.GetGameMode`) :!pure true))
    (bind _aspch_game (cast `/Game/Assets/Gameplay/PCH_Game` (`self.K2_GetPawn` _array_element)))
    (`KismetArrayLibrary.Array_Add` (`local.Names`) (`/Game/Assets/Gameplay/PCH_Game.PlayerName` _aspch_game))
    (`KismetArrayLibrary.Array_Add` (`local.IDs`) (`/Game/Assets/Gameplay/PCH_Game.PlayerID` _aspch_game)))
  (for _array_element_2 (`/Game/Assets/Gameplay/GM_Lobby.PcList` (cast `/Game/Assets/Gameplay/GM_Lobby` (`GameplayStatics.GetGameMode`) :!pure true))
    (`self.EVE_Client_Update_Player` _array_element_2 (`local.Names`) (`local.IDs`))))

(fn `UserConstructionScript`)