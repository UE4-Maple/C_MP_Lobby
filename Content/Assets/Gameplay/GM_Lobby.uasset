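; GM_Lobby is the lobby game mode, keeping a list of connected PC_Lobby player controllers.
; PostLogin adds each controller uniquely, while OnLogout removes it and calls FUNUpdatePlayer on player controller 0.
; FUNFindPCByID searches the list for the controller whose PCH_Game pawn has a matching PlayerID, stopping early if a pawn fails that cast.
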(event `self.K2_PostLogin`
  (params (NewPlayer :type "PlayerController Object Reference"))
  (bind _aspc_lobby (cast `/Game/Assets/Gameplay/PC_Lobby` NewPlayer))
  (`KismetArrayLibrary.Array_AddUnique` (`self.PcList`) _aspc_lobby))

(event `self.K2_OnLogout`
  (params (ExitingController :type "Controller Object Reference"))
  (bind _aspc_lobby (cast `/Game/Assets/Gameplay/PC_Lobby` ExitingController))
  (`KismetArrayLibrary.Array_RemoveItem` (`self.PcList`) _aspc_lobby)
  (bind _aspc_lobby_2 (cast `/Game/Assets/Gameplay/PC_Lobby` (`GameplayStatics.GetPlayerController` 0)))
  (`/Game/Assets/Gameplay/PC_Lobby.FUN_Update_Player` _aspc_lobby_2))

(fn `FUN_Find_PC_ByID`
  (params (Id :type String))
  (returns (PC :type "/Game/Assets/Gameplay/PC_Lobby Object Reference"))
  (for _array_element (`self.PcList`)
    (bind _aspch_game (cast `/Game/Assets/Gameplay/PCH_Game` (`Controller.K2_GetPawn` _array_element)))
    (if (`KismetStringLibrary.EqualEqual_StrStr` (`/Game/Assets/Gameplay/PCH_Game.PlayerID` _aspch_game) Id)
      (return _array_element))))

(fn `UserConstructionScript`)