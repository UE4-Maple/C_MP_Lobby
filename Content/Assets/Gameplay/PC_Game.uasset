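; Player controller for gameplay that spawns and possesses the player's PCH_Game pawn.
; On BeginPlay, the local controller reads the player name and index from GI_Main and passes them to its spawn event.
; That event spawns the pawn at the single PlayerStart returned by GetActorOfClass, with a PlayerID built by concatenating current date and time down to milliseconds.
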(event `self.ReceiveBeginPlay`
  (if (`self.IsLocalPlayerController`)
    (bind _asgi_main (cast `/Game/Assets/Gameplay/GI_Main` (`GameplayStatics.GetGameInstance`)))
    (`self.EVE_Spawn_Player` (`/Game/Assets/Gameplay/GI_Main.PlayerName` _asgi_main) (`/Game/Assets/Gameplay/GI_Main.PlayerIndex` _asgi_main))))

(event `EVE_Spawn_Player`
  (params (PlayerName :type Text) (PlayerIndex :type Integer))
  (bind (_returnvalue_year _returnvalue_month _returnvalue_day _returnvalue_hour _returnvalue_minute _returnvalue_second _returnvalue_millisecond) (`KismetMathLibrary.BreakDateTime` (`KismetMathLibrary.Now`)))
  (bind _returnvalue (`GameplayStatics.GetActorOfClass` "/Script/Engine.PlayerStart"))
  (bind _returnvalue_2 (`|SpawnActorFromClass` "/Game/Assets/Gameplay/PCH_Game.PCH_Game_C" (`self.GetTransform` _returnvalue) "Undefined" "OverrideRootScale" null (`KismetStringLibrary.Concat_StrStr` (`KismetStringLibrary.Conv_IntToString` _returnvalue_year) (`KismetStringLibrary.Conv_IntToString` _returnvalue_month) (`KismetStringLibrary.Conv_IntToString` _returnvalue_day) (`KismetStringLibrary.Conv_IntToString` _returnvalue_hour) (`KismetStringLibrary.Conv_IntToString` _returnvalue_minute) (`KismetStringLibrary.Conv_IntToString` _returnvalue_second) (`KismetStringLibrary.Conv_IntToString` _returnvalue_millisecond)) PlayerName PlayerIndex null))
  (`self.Possess` self _returnvalue_2))

(fn `UserConstructionScript`)